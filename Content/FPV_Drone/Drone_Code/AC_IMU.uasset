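; Drone IMU component that simulates inertial sensor readings from a target actor's motion.
; Each Tick it derives rotation rates in radians per second and acceleration by finite differences against cached values, then broadcasts them with velocity through SendIMUData.
; Roll change feeds the YawRate output and yaw change feeds RollRate.
; The cache setters are separate functions that Tick does not call.
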(event EventBeginPlay)

(event EventTick
  (params (DeltaSeconds :type Float%20%28single-precision%29))
  (bind _targetarctor (Variables|Default|GetTargetArctor))
  (bind _targetarctor_2 (Variables|Default|GetTargetArctor))
  (bind _returnvalue (Transformation|GetVelocity _targetarctor))
  (bind _returnvalue_2 (Transformation|GetActorTransform _targetarctor_2))
  (bind (_rotationratex _rotationratey _rotationratez) (CallFunction|CalculateRotationRate (.roll (.rotation _returnvalue_2)) (.pitch (.rotation _returnvalue_2)) (.yaw (.rotation _returnvalue_2)) DeltaSeconds))
  (bind _acceleration (CallFunction|CalculateAcceleration DeltaSeconds (Variables|Default|GetCached_Velocity) _returnvalue))
  (Default|CallSendIMUData (Utilities|Struct|MakeIMU_Data _rotationratex _rotationratey _rotationratez _acceleration _returnvalue)))

(fn SetCacheRotationRate
  (bind _targetarctor (Variables|Default|GetTargetArctor))
  (bind _returnvalue (Transformation|GetActorTransform _targetarctor))
  (Variables|Default|SetCached_X (.roll (.rotation _returnvalue)))
  (Variables|Default|SetCached_Y (.pitch (.rotation _returnvalue)))
  (Variables|Default|SetCached_Z (.yaw (.rotation _returnvalue))))

(fn SetCacheVelocity
  (Variables|Default|SetCached_Velocity (Transformation|GetVelocity (Variables|Default|GetTargetArctor))))

(fn CalculateRotationRateSingle
  (params (NewRotation :type Float%20%28double-precision%29) (CachedRotation :type Float%20%28double-precision%29) (DeltaTime :type Float%20%28double-precision%29))
  (return (/ (Math|Trig|DegreesToRadians (- NewRotation CachedRotation)) DeltaTime)))

(fn CalculateRotationRate
  (params (NewRotationX :type Float%20%28double-precision%29) (NewRotationY :type Float%20%28double-precision%29) (NewRotationZ :type Float%20%28double-precision%29) (DeltaTime :type Float%20%28single-precision%29))
  (return (CallFunction|CalculateRotationRateSingle NewRotationX (Variables|Default|GetCached_X) DeltaTime) (CallFunction|CalculateRotationRateSingle NewRotationY (Variables|Default|GetCached_Y) DeltaTime) (CallFunction|CalculateRotationRateSingle NewRotationZ (Variables|Default|GetCached_Z) DeltaTime)))

(fn CalculateAcceleration
  (params (DeltaTime :type Float%20%28double-precision%29) (CacheVelocity :type Vector) (NewVelocity :type Vector))
  (return (/ (- NewVelocity CacheVelocity) DeltaTime)))