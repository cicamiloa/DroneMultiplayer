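; BP_Flower is a marker actor that a drone collects once by flying into its box.
; On BeginPlay it passes its world location to its Widget_Marker widget as the marker's origin.
; While IsActive is set, an overlapping SimpleDrone gets a FlowerOverlap call, then the flower hides its widget and deactivates itself.
; Every box overlap also prints a debug string, whatever the actor or state.
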(event OnComponentBeginOverlap(Box)
  (params (OverlappedComponent :type Primitive%20Component%20Object%20Reference) (OtherActor :type Actor%20Object%20Reference) (OtherComp :type Primitive%20Component%20Object%20Reference) (OtherBodyIndex :type Integer) (bFromSweep :type Boolean) (SweepResult :type Hit%20Result%20Structure%20%28by%20ref%29))
  (Development|PrintString "Hello")
  (if (Variables|Default|GetIsActive)
    (bind _assimple_drone (Utilities|Casting|CastToSimpleDrone OtherActor))
    (Default|FlowerOverlap _assimple_drone)
    (Rendering|SetVisibility (Variables|Default|GetWidget) false false)
    (Variables|Default|SetIsActive false)))

(event EventBeginPlay
  (bind _aswidget_marker (Utilities|Casting|CastToWidget_Marker (UserInterface|GetWidget (Variables|Default|GetWidget))))
  (Variables|/Game/Drone/Markers/Widget_Marker.Widget_Marker_C|SetOriginLocation _aswidget_marker (Transformation|GetActorLocation)))

(fn ConstructionScript)